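; Locked door Blueprint that the player can open and close with the interact input once they hold a key.
; The Doorbox overlap shows an Interactprompt widget, enables input and opens a gate while the first-person character is inside, reversing this on exit.
; Interact briefly flags the prompt as pressed, then, if Haskey is true, a FlipFlop plays or reverses a timeline that lerps the mesh yaw between closed and open angles.
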(event `InputAction|interact`
  (params (Key :type "Key Structure"))
  (:`Pressed`
    (set `/Game/widget/interactprompt.is pressed` true (stale `self.doorbox.OnComponentBeginOverlap` _returnvalue))
    (`KismetSystemLibrary.Delay` 0.2)
    (set `/Game/widget/interactprompt.is pressed` false (stale `self.doorbox.OnComponentBeginOverlap` _returnvalue))
    (if (`/Game/FirstPersonBP/Blueprints/FirstPersonCharacter.haskey?` (stale `self.doorbox.OnComponentBeginOverlap` _asfirst_person_character))
      (`/Engine/EditorBlueprintResources/StandardMacros.Gate` true :!label _label
        (:`Exit`
          ;[1 1 1] open/close door animation
          (`/Engine/EditorBlueprintResources/StandardMacros.FlipFlop`
            (:`A`
              (bind (_direction _door_track) (`Timeline|open/close door` :!label _label_2)
                (:`Update`
                  (`SceneComponent.K2_SetRelativeRotation` (`self.StaticMesh`) (`KismetMathLibrary.MakeRotator` 0.0 0.0 (`KismetMathLibrary.Lerp` (`self.closed angle`) (`self.open angle`) _door_track)) false false))))
            (:`B`
              (goto _label_2 :!via `Reverse`))))))))

(event `self.doorbox.OnComponentBeginOverlap`
  (params (OverlappedComponent :type "PrimitiveComponent Object Reference") (OtherActor :type "Actor Object Reference") (OtherComp :type "PrimitiveComponent Object Reference") (OtherBodyIndex :type Integer) (bFromSweep :type Boolean) (SweepResult :type "HitResult Structure (by ref)"))
  (bind _asfirst_person_character (cast `/Game/FirstPersonBP/Blueprints/FirstPersonCharacter` OtherActor))
  (bind _returnvalue (`|CreateWidget` "/Game/widget/interactprompt.interactprompt_C"))
  (`UserWidget.AddToViewport` _returnvalue 0)
  (`self.EnableInput` (`GameplayStatics.GetPlayerController` 0))
  (goto _label :!via `Open`))

(event `self.doorbox.OnComponentEndOverlap`
  (params (OverlappedComponent :type "PrimitiveComponent Object Reference") (OtherActor :type "Actor Object Reference") (OtherComp :type "PrimitiveComponent Object Reference") (OtherBodyIndex :type Integer))
  (cast `/Game/FirstPersonBP/Blueprints/FirstPersonCharacter` OtherActor)
  (`Widget.RemoveFromParent` (stale `self.doorbox.OnComponentBeginOverlap` _returnvalue))
  (`self.DisableInput` (`GameplayStatics.GetPlayerController` 0))
  (goto _label :!via `Close`))

(fn `UserConstructionScript`)